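; Knight player character Blueprint that picks up items and handles arming, disarming and melee attacks through Enhanced Input.
; Capsule overlaps track the nearby BP_Item, which the Equip input snaps to the right-hand socket.
; A PlayerActionState gate lets Arm toggle equip montage sections for a valid Weapon and Attack play a random montage section when armed.
; The return to Idle after either action is not handled in these graphs.
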(event Custom|OnComponentBeginOverlap_Event
  (params (OverlappedComponent :type Primitive%20Component%20Object%20Reference) (OtherActor :type Actor%20Object%20Reference) (OtherComp :type Primitive%20Component%20Object%20Reference) (OtherBodyIndex :type Integer) (bFromSweep :type Boolean) (SweepResult :type Hit%20Result%20Structure%20%28by%20ref%29))
  ;[0.15 0 0.1236 0.5] Bind sphere collider to event
  (bind _asbp_item (Utilities|Casting|CastToBP_Item OtherActor))
  (Variables|Default|SetCollidedItem _asbp_item))

(event Custom|OnComponentEndOverlap_Event
  (params (OverlappedComponent :type Primitive%20Component%20Object%20Reference) (OtherActor :type Actor%20Object%20Reference) (OtherComp :type Primitive%20Component%20Object%20Reference) (OtherBodyIndex :type Integer))
  ;[0.15 0 0.1236 0.5] Bind sphere collider to event
  (bind _asbp_item (Utilities|Casting|CastToBP_Item OtherActor))
  (if (== _asbp_item (Variables|Default|GetCollidedItem))
    (Variables|Default|SetCollidedItem 0)))

(event Input|EnhancedActionEvents|EnhancedInputActionIA_Equip
  (params (ActionValue :type Boolean) (ElapsedSeconds :type Float%20%28double-precision%29) (TriggeredSeconds :type Float%20%28double-precision%29) (InputAction :type Input%20Action%20Object%20Reference :default "/Game/Blueprints/Input/Actions/IA_Equip.IA_Equip"))
  (bind _collideditem (Variables|Default|GetCollidedItem))
  (:Started
    (Utilities|IsValid _collideditem
      (:Is%20Valid
        (Transformation|AttachComponentToComponent (Variables|/Game/Blueprints/Items/BP_Item.BP_Item_C|GetItem _collideditem) (Variables|Character|GetMesh) "RightHandSocket" "SnapToTarget" "SnapToTarget" "KeepRelative" true)
        (Variables|/Game/Blueprints/Items/BP_Item.BP_Item_C|SetIsEquipped (Variables|Default|GetCollidedItem) true)
        (Default|EquipItem (Variables|Default|GetCollidedItem))))))

(event Input|EnhancedActionEvents|EnhancedInputActionIA_Attack
  (params (ActionValue :type Boolean) (ElapsedSeconds :type Float%20%28double-precision%29) (TriggeredSeconds :type Float%20%28double-precision%29) (InputAction :type Input%20Action%20Object%20Reference :default "/Game/Blueprints/Input/Actions/IA_Attack.IA_Attack"))
  (:Started
    (if (Utilities|Enum|Equal(Enum) (Variables|Default|GetPlayerActionState) "EPAS_Idle")
      (if (Variables|Default|GetIsArmed)
        (Animation|PlayAnimMontage "/Game/Animations/AM_Attack.AM_Attack" 1.0 (CallFunction|GetRandomAttackMontageSection))
        (Variables|Default|SetPlayerActionState "EPAS_Attacking")))))

(event Input|EnhancedActionEvents|EnhancedInputActionIA_Arm
  (params (ActionValue :type Boolean) (ElapsedSeconds :type Float%20%28double-precision%29) (TriggeredSeconds :type Float%20%28double-precision%29) (InputAction :type Input%20Action%20Object%20Reference :default "/Game/Blueprints/Input/Actions/IA_Arm.IA_Arm"))
  (:Started
    (Utilities|IsValid (Variables|Default|GetWeapon)
      (:Is%20Valid
        (if (Utilities|Enum|Equal(Enum) "EPAS_Idle" (Variables|Default|GetPlayerActionState))
          (if (Variables|Default|GetIsArmed)
            (Animation|PlayAnimMontage "/Game/Animations/AM_Equip.AM_Equip" 1.0 "Disarm")
            (Variables|Default|SetIsArmed false)
            (else
              (Animation|PlayAnimMontage "/Game/Animations/AM_Equip.AM_Equip" 1.0 "Arm")
              (Variables|Default|SetIsArmed true)))
          (Variables|Default|SetPlayerActionState "EPAS_Arming"))))))

(event EventBeginPlay
  ;[0.15 0 0.1236 0.5] Bind sphere collider to event
  (Collision|AssignOnComponentBeginOverlap (Variables|Default|GetCapsuleComponent) (delegate Custom|OnComponentBeginOverlap_Event))
  (Collision|AssignOnComponentEndOverlap (Variables|Default|GetCapsuleComponent) (delegate Custom|OnComponentEndOverlap_Event))
  (Variables|Default|SetPlayerActionState "EPAS_Idle"))

(fn ConstructionScript)

(fn GetRandomAttackMontageSection
  (bind _attackmontagesections (Variables|Default|GetAttackMontageSections))
  (return (Utilities|String|StringToName (Utilities|Array|Get(acopy) _attackmontagesections (Math|Random|RandomInteger (Utilities|Array|Length _attackmontagesections))))))
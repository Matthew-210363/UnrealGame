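; BP_Item is an item actor that moves vertically on a sine wave.
; BeginPlay sets TimeConstant, and Tick feeds TransformedSine, defined outside this Blueprint, into the Z of a per-frame world offset.
; An overlap handler only prints and logs test messages, with no binding shown.
; Debug print and sphere nodes are left disconnected, and TransformedCos is unused.
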(event Custom|OnActorBeginOverlap_Event
  (params (OverlappedActor :type Actor%20Object%20Reference) (OtherActor :type Actor%20Object%20Reference))
  (Development|PrintString "Hello from the other side")
  (Utilities|String|LogString "BP log"))

(event EventBeginPlay
  (Variables|Default|SetTimeConstant 5.0))

(event Collision|EventActorBeginOverlap
  (params (OtherActor :type Actor%20Object%20Reference)))

(event EventTick
  (params (DeltaSeconds :type Float%20%28single-precision%29))
  (bind _returnvalue (Class|Item|TransformedSine))
  (Transformation|AddActorWorldOffset (Math|Vector|MakeVector 0.0 0.0 _returnvalue)))

(fn ConstructionScript)